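; Rotating wall actor that spins continuously around the yaw axis of its Center component.
; BeginPlay starts an endless 0.016-second Delay loop that adds RotationRate to the local yaw on each pass, in place of Tick or delta-time scaling.
; The construction script shapes the wall by offsetting ScalePoint down local Z by Distance and setting its Y scale to HightScale.
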(event EventBeginPlay
  (Utilities|FlowControl|Delay 0.016 :!label _label)
  (Transformation|AddLocalRotation (Variables|Default|GetCenter) (Math|Rotator|MakeRotator 0.0 0.0 (Variables|Default|GetRotation%20Rate)) false false)
  (goto _label))

(fn ConstructionScript
  (Transformation|AddLocalOffset (Variables|Default|GetScale_Point) (Math|Vector|MakeVector 0.0 0.0 (* -1 (Variables|Default|GetDistance))) false false)
  (Transformation|SetRelativeScale3D (Variables|Default|GetScale_Point) (Math|Vector|MakeVector 1.0 (Variables|Default|GetHight_Scale) 1.0)))