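; Shield_Box is a pickup that restores a Ghost_Player's shield on overlap, only if it is not already ready.
; A one-time trigger sets ShieldReady, plays a sound and the GUI recharge animation, then runs a timeline driving cube scale and light intensity before destroying the actor.
; A replayed idle timeline bobs, pulses and spins the cube, with a random rotation rate chosen at BeginPlay.
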(event OnComponentBeginOverlap(Box)
  (params (OverlappedComponent :type Primitive%20Component%20Object%20Reference) (OtherActor :type Actor%20Object%20Reference) (OtherComp :type Primitive%20Component%20Object%20Reference) (OtherBodyIndex :type Integer) (bFromSweep :type Boolean) (SweepResult :type Hit%20Result%20Structure%20%28by%20ref%29))
  (bind _asghost_player (Utilities|Casting|CastToGhost_Player OtherActor))
  (if (not (Variables|/Game/Blueprints/Ghost_Player.Ghost_Player_C|GetShield_Ready _asghost_player))
    (Utilities|FlowControl|DoOnce false
      (:Completed
        (Variables|/Game/Blueprints/Ghost_Player.Ghost_Player_C|SetShield_Ready _asghost_player true)
        (Audio|PlaySound2D "/Game/Effects/Audio/Cue_Shield.Cue_Shield" 1.0 3.0 0.75 0 0)
        (Default|PlayShieldRecharge (Variables|/Game/Blueprints/Ghost_Player.Ghost_Player_C|GetGUI _asghost_player))
        (bind _alpha (Timeline|Timeline_0 PlayFromStart)
          (:Update
            (Transformation|SetRelativeScale3D (Variables|Default|GetCube) (Math|Vector|MakeVector (* _alpha 1.0) (* _alpha 1.0) (* _alpha 1.0)))
            (Rendering|Components|Light|SetIntensity (Variables|Default|GetPointLight) (* _alpha 3e+02)))
          (:Finished
            (Actor|DestroyActor)))))))

(event Custom|Replay_Anim
  (bind _cube (Variables|Default|GetCube))
  (bind _alpha (Timeline|Idle_Animation_Timeline PlayFromStart)
    (:Update
      (Transformation|SetRelativeLocation _cube (Math|Vector|MakeVector 0.0 0.0 (+ (* _alpha 1e+01) 5e+01)) false false)
      (Transformation|SetRelativeScale3D _cube (Math|Vector|MakeVector (+ (* _alpha 0.03) 1.0) (+ (* _alpha 0.03) 1.0) (+ (* _alpha 0.03) 1.0)))
      (Transformation|AddRelativeRotation _cube (Math|Rotator|MakeRotator 0.0 0.0 (Variables|Default|GetRotation_Rate)) false false))
    (:Finished
      (CallFunction|ReplayAnim))))

(event EventBeginPlay
  (bind _cube (Variables|Default|GetCube))
  (Variables|Default|SetRotation_Rate (Math|Random|RandomFloatinRange 0.7 1.3))
  (bind _alpha (Timeline|Idle_Animation_Timeline PlayFromStart)
    (:Update
      (Transformation|SetRelativeLocation _cube (Math|Vector|MakeVector 0.0 0.0 (+ (* _alpha 1e+01) 5e+01)) false false)
      (Transformation|SetRelativeScale3D _cube (Math|Vector|MakeVector (+ (* _alpha 0.03) 1.0) (+ (* _alpha 0.03) 1.0) (+ (* _alpha 0.03) 1.0)))
      (Transformation|AddRelativeRotation _cube (Math|Rotator|MakeRotator 0.0 0.0 (Variables|Default|GetRotation_Rate)) false false))
    (:Finished
      (CallFunction|ReplayAnim))))

(fn ConstructionScript)