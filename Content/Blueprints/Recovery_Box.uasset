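; Recovery box pickup that calls Recover on a Ghost_Player overlapping it, only if that player's GotHit flag is set.
; A timeline started on BeginPlay bobs, pulses and spins the Scene component, replaying itself on finish for a looping idle animation.
; On pickup, a disappear timeline animates the Scene scale and point light intensity, then destroys the actor.
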(event OnComponentBeginOverlap(Box)
  (params (OverlappedComponent :type Primitive%20Component%20Object%20Reference) (OtherActor :type Actor%20Object%20Reference) (OtherComp :type Primitive%20Component%20Object%20Reference) (OtherBodyIndex :type Integer) (bFromSweep :type Boolean) (SweepResult :type Hit%20Result%20Structure%20%28by%20ref%29))
  (bind _asghost_player (Utilities|Casting|CastToGhost_Player OtherActor))
  (if (Variables|/Game/Blueprints/Ghost_Player.Ghost_Player_C|GetGot_Hit _asghost_player)
    (Default|Recover _asghost_player)
    (bind _alpha (Timeline|Dissappear_Timeline PlayFromStart)
      (:Update
        (Transformation|SetRelativeScale3D (Variables|Default|GetScene) (Math|Vector|MakeVector (* _alpha 0.8) (* _alpha 0.8) (* _alpha 0.8)))
        (Rendering|Components|Light|SetIntensity (Variables|Default|GetPointLight) (* _alpha 3e+02)))
      (:Finished
        (Actor|DestroyActor)))))

(event Custom|Replay_Anim
  (bind _scene (Variables|Default|GetScene))
  (bind _alpha (Timeline|Timeline_0 PlayFromStart)
    (:Update
      (Transformation|SetRelativeLocation _scene (Math|Vector|MakeVector 0.0 0.0 (+ (* _alpha 1e+01) 2e+01)) false false)
      (Transformation|SetRelativeScale3D _scene (Math|Vector|MakeVector (+ (* _alpha 0.03) 0.8) (+ (* _alpha 0.03) 0.8) (+ (* _alpha 0.03) 0.8)))
      (Transformation|AddRelativeRotation _scene (Math|Rotator|MakeRotator 0.0 0.0 1.0) false false))
    (:Finished
      (CallFunction|ReplayAnim))))

(event EventBeginPlay
  (bind _scene (Variables|Default|GetScene))
  (bind _alpha (Timeline|Timeline_0 PlayFromStart)
    (:Update
      (Transformation|SetRelativeLocation _scene (Math|Vector|MakeVector 0.0 0.0 (+ (* _alpha 1e+01) 2e+01)) false false)
      (Transformation|SetRelativeScale3D _scene (Math|Vector|MakeVector (+ (* _alpha 0.03) 0.8) (+ (* _alpha 0.03) 0.8) (+ (* _alpha 0.03) 0.8)))
      (Transformation|AddRelativeRotation _scene (Math|Rotator|MakeRotator 0.0 0.0 1.0) false false))
    (:Finished
      (CallFunction|ReplayAnim))))

(fn ConstructionScript)