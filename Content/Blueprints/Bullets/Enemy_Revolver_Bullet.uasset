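; Enemy revolver bullet that damages the player or rewards them for shielded hits and close passes.
; Tick grants one point without streak, once per bullet, when the Ghost_Player comes within a short range.
; OnImpact spawns an effect oriented along the incoming velocity, then either awards streak points if the struck player's shield is active or calls GetHit.
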(event EventOnImpact
  (params (Ricochet :type Boolean) (PassedThrough :type Boolean) (Location :type Vector :default "0, 0, 0") (IncomingVelocity :type Vector :default "0, 0, 0") (Normal :type Vector :default "0, 0, 0") (ExitLocation :type Vector :default "0, 0, 0") (ExitVelocity :type Vector :default "0, 0, 0") (Impulse :type Vector :default "0, 0, 0") (PenetrationDepth :type Float%20%28single-precision%29) (Actor :type Actor%20Object%20Reference) (Component :type Scene%20Component%20Object%20Reference) (BoneName :type Name :default "None") (PhysMaterial :type Physical%20Material%20Object%20Reference) (HitResult :type Hit%20Result%20Structure))
  (Niagara|SpawnSystematLocation "/Game/Effects/Impact_System.Impact_System" Location (Math|Rotator|FindLookatRotation Location (+ Location IncomingVelocity)))
  (bind _asghost_player (Utilities|Casting|CastToGhost_Player Actor))
  (if (Variables|/Game/Blueprints/Ghost_Player.Ghost_Player_C|GetShield_Active _asghost_player)
    (Default|AddPoints _asghost_player 9 true)
    (else
      (Default|GetHit _asghost_player))))

(event EventTick
  (params (DeltaSeconds :type Float%20%28single-precision%29))
  (bind _returnvalue (Game|GetPlayerCharacter 0))
  (bind _asghost_player (Utilities|Casting|CastToGhost_Player _returnvalue))
  (if (< (Transformation|GetDistanceTo _returnvalue self) 2e+02)
    (Utilities|FlowControl|DoOnce false
      (:Completed
        (Default|AddPoints _asghost_player 1 false)))))

(fn ConstructionScript)