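; Revolver bullet that resolves its impact as either an enemy kill or a miss for the Ghost_Player.
; Hitting a Base_Enemy or Melee_Enemy makes it self-destruct and charges the player's dash.
; A miss spawns an impact effect offset and oriented by velocity and surface normal, breaks the streak and deducts points.
; Every impact also spawns a trail effect aligned with the incoming velocity.
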(event EventOnImpact
  (params (Ricochet :type Boolean) (PassedThrough :type Boolean) (Location :type Vector :default "0, 0, 0") (IncomingVelocity :type Vector :default "0, 0, 0") (Normal :type Vector :default "0, 0, 0") (ExitLocation :type Vector :default "0, 0, 0") (ExitVelocity :type Vector :default "0, 0, 0") (Impulse :type Vector :default "0, 0, 0") (PenetrationDepth :type Float%20%28single-precision%29) (Actor :type Actor%20Object%20Reference) (Component :type Scene%20Component%20Object%20Reference) (BoneName :type Name :default "None") (PhysMaterial :type Physical%20Material%20Object%20Reference) (HitResult :type Hit%20Result%20Structure))
  ;[1 1 1] Impact particles
  (Utilities|FlowControl|Sequence
    (:then_0
      (bind _asbase_enemy (Utilities|Casting|CastToBase_Enemy Actor)
        (:then
          (Default|SelfDistruct _asbase_enemy)
          (bind _asghost_player (Utilities|Casting|CastToGhost_Player (Game|GetPlayerCharacter 0) :!label _label))
          (Default|ChargeDash _asghost_player 100))
        (:CastFailed
          (bind _asmelee_enemy (Utilities|Casting|CastToMelee_Enemy Actor)
            (:then
              (Default|SelfDistruct _asmelee_enemy)
              (goto _label))
            (:CastFailed
              ;[1 1 1] Impact on miss
              (Niagara|SpawnSystematLocation "/Game/Effects/Impact_System.Impact_System" (+ (/ IncomingVelocity -6e+02) (* Normal 25.0) Location) (Math|Rotator|FindLookatRotation Location (+ Location IncomingVelocity (* Normal -5e+02))) "0.800000,0.800000,0.800000")
              (bind _asghost_player_2 (Utilities|Casting|CastToGhost_Player (Game|GetPlayerCharacter 0)))
              (Default|BreakStreak _asghost_player_2)
              (Default|AddPoints _asghost_player_2 -2 true))))))
    (:then_1
      (Niagara|SpawnSystematLocation "/Game/Effects/Impact_System_Trail.Impact_System_Trail" Location (Math|Rotator|FindLookatRotation Location (+ Location IncomingVelocity))))))

(fn ConstructionScript)