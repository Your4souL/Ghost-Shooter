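; Obsolete turret Blueprint that aims at the player and shoots while they are within range.
; A Delay loop started on BeginPlay polls the distance ten times a second instead of using Tick, toggling Shoot on Turret.
; In range, RotationPoint turns toward a point slightly below the player's location.
; The RInterpTo call uses fixed delta time and speed values that make each update snap straight to the target rotation.
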(event EventBeginPlay
  (bind _returnvalue (Game|GetPlayerCharacter 0))
  (bind _rotation_point (Variables|Default|GetRotation_Point))
  (bind _rotation_point_2 (Variables|Default|GetRotation_Point))
  (bind _returnvalue_2 (Transformation|GetWorldLocation _rotation_point_2))
  (bind _returnvalue_3 (Transformation|GetActorLocation _returnvalue))
  (bind _returnvalue_4 (+ _returnvalue_3 "0, 0,-50.000000"))
  (if (<= (Transformation|GetDistanceTo _returnvalue) 1e+03) :!label _label
    (Transformation|SetWorldRotation _rotation_point (Math|Interpolation|RInterpTo (Transformation|GetWorldRotation _rotation_point) (Math|Rotator|FindLookatRotation (Math|Vector|MakeVector (.x _returnvalue_2) (.y _returnvalue_2) (.z _returnvalue_2)) (Math|Vector|MakeVector (.x _returnvalue_4) (.y _returnvalue_4) (.z _returnvalue_4))) 1.0 1.0) false false)
    (Class|EBBarrel|Shoot (Variables|Default|GetTurret) true)
    (else
      (Class|EBBarrel|Shoot (Variables|Default|GetTurret) false)))
  (Utilities|FlowControl|Delay 0.1)
  (goto _label))

(fn ConstructionScript)