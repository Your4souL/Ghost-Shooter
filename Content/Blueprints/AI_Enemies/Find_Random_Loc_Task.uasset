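; Behavior tree task that picks a movement destination for an AI enemy and writes it to a Blackboard vector key.
; Melee_Enemy pawns get the player character's current location, while any other pawn gets a random navigable point near itself.
; Both branches finish successfully at once, leaving the movement itself outside this task.
; Focus-clearing and guard-point wandering nodes remain in the graph but are unused.
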(event EventReceiveExecuteAI
  (params (OwnerController :type AI%20Controller%20Object%20Reference) (ControlledPawn :type Pawn%20Object%20Reference))
  (bind _asmelee_enemy (Utilities|Casting|CastToMelee_Enemy ControlledPawn)
    (:then
      (AI|BehaviorTree|SetBlackboardValueasVector (Variables|Default|GetBB_Move_Target_Key) (Transformation|GetActorLocation (Game|GetPlayerCharacter 0)))
      (AI|BehaviorTree|FinishExecute true))
    (:CastFailed
      (AI|BehaviorTree|SetBlackboardValueasVector (Variables|Default|GetBB_Move_Target_Key) (.RandomLocation (Class|NavigationSystemV1|GetRandomPointinNavigableRadius (Transformation|GetActorLocation ControlledPawn) 5e+02 0 0)))
      (AI|BehaviorTree|FinishExecute true))))