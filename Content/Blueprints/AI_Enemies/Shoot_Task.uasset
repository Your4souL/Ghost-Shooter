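; Behavior tree task that triggers an AI enemy's attack based on the type of the controlled pawn.
; A Base_Enemy calls Shoot and succeeds immediately, with no range check.
; A Melee_Enemy calls Hit and succeeds if the Ghost_Player is within a fixed distance, otherwise it calls EndHit and fails.
; Any failed cast also ends the task as failed.
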(event EventReceiveExecuteAI
  (params (OwnerController :type AI%20Controller%20Object%20Reference) (ControlledPawn :type Pawn%20Object%20Reference))
  (bind _asbase_enemy (Utilities|Casting|CastToBase_Enemy ControlledPawn)
    (:then
      (Default|Shoot _asbase_enemy)
      (AI|BehaviorTree|FinishExecute true :!label _label))
    (:CastFailed
      (bind _asmelee_enemy (Utilities|Casting|CastToMelee_Enemy ControlledPawn)
        (:then
          (bind _asghost_player (Utilities|Casting|CastToGhost_Player (Game|GetPlayerCharacter 0))
            (:then
              (if (<= (Math|Vector|Distance(Vector) (Transformation|GetActorLocation _asghost_player) (Transformation|GetActorLocation _asmelee_enemy)) 1e+03)
                (Default|Hit _asmelee_enemy)
                (goto _label)
                (else
                  (Default|EndHit _asmelee_enemy))))
            (:CastFailed
              _)))
        (:CastFailed
          _))
      (AI|BehaviorTree|FinishExecute false))))