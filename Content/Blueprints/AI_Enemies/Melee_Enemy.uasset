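; Melee enemy character that leaps and dashes at the player, with an Elite variant that dashes faster, leads player movement and has its own look.
; Hit launches it upward, then toward the player, opening a gate on a looping overlap check of KillingCapsule.
; Contact hurts the player or awards points if shielded; afterwards the AI controller's state updates.
; Self-destruct plays effects and grants points, streak and revolver charge.
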(event Custom|Hit
  (bind _returnvalue (Game|GetPlayerCharacter 0))
  (bind _returnvalue_2 (Game|GetPlayerCharacter 0))
  (bind _mesh (Variables|Character|GetMesh))
  (bind _mesh_2 (Variables|Character|GetMesh))
  (bind _hit_system (Variables|Default|GetHit_System))
  (bind _elite (Variables|Default|GetElite))
  (bind _returnvalue_3 (Transformation|GetActorLocation _returnvalue_2))
  (bind _returnvalue_4 (Utilities|IsValid _returnvalue_2))
  (bind _returnvalue_5 (Transformation|GetWorldLocation _mesh_2))
  (bind _returnvalue_6 (Transformation|GetVelocity _returnvalue_2))
  (bind _returnvalue_7 (Transformation|GetWorldLocation _mesh))
  (bind _returnvalue_8 (select _elite 0.15 0.0))
  (bind _returnvalue_9 (* _returnvalue_6 _returnvalue_8))
  (bind _returnvalue_10 (+ _returnvalue_3 _returnvalue_9))
  (bind _returnvalue_11 (Math|Vector|SelectVector _returnvalue_10 _returnvalue_5 _returnvalue_4))
  (bind _returnvalue_12 (- _returnvalue_5 _returnvalue_11))
  ;[1 1 1] Hit
  (Components|Activation|Activate _hit_system false)
  (Utilities|IsValid self
    (:Is%20Valid
      (Character|LaunchCharacter "0, 0,1700.000000" false true)
      (Utilities|FlowControl|Delay 0.3)
      (Utilities|IsValid self
        (:Is%20Valid
          (Audio|PlaySoundatLocation "/Game/Effects/Audio/Cue_Dash.Cue_Dash" (Transformation|GetActorLocation) "0, 0, 0" 1.0 3.0 0.0 "/Game/Effects/Audio/Base_Dir_Attenuation.Base_Dir_Attenuation" 0 0)
          (Character|LaunchCharacter (* (Math|Vector|Normalize (Math|Vector|MakeVector (.x _returnvalue_12) (.y _returnvalue_12) (/ (Math|Vector|Distance(Vector) _returnvalue_7 (Math|Vector|SelectVector (Transformation|GetActorLocation _returnvalue) _returnvalue_7 (Utilities|IsValid _returnvalue))) (select (Variables|Default|GetElite) -6.0 -4.0)))) (select (Variables|Default|GetElite) -5e+03 -3.5e+03)) true true)
          (Utilities|FlowControl|Sequence
            (:then_0
              (Utilities|FlowControl|Gate true) ; enters at Open
            )
            (:then_1
              (Utilities|FlowControl|Delay 0.3)
              (Components|Activation|Deactivate _hit_system)
              (bind _asbase_enemy_controller (Utilities|Casting|CastToBase_Enemy_Controller (Pawn|GetController)))
              (Variables|/Game/Blueprints/AI_Enemies/Base_Enemy_Controller.Base_Enemy_Controller_C|SetState _asbase_enemy_controller "NewEnumerator0")
              (Default|UpdateState _asbase_enemy_controller))))))))

(event Custom|Update_Gun
  (params (New_Rotation :type Rotator))
  (Transformation|SetWorldRotation (Variables|Default|GetGun_Rotation_Point) New_Rotation false false))

(event Custom|Self_Distruct
  (bind _mesh (Variables|Character|GetMesh))
  (bind _returnvalue (Transformation|GetWorldLocation _mesh))
  ;[1 1 1] Death
  (Audio|PlaySoundatLocation "/Game/Effects/Audio/Soul_Pha_Cue.Soul_Pha_Cue" _returnvalue "0, 0, 0" 1.0 1.0 0.0 "/Game/Effects/Audio/Base_Dir_Attenuation.Base_Dir_Attenuation" 0 0)
  (Niagara|SpawnSystematLocation "/Game/Effects/Melee_Enemy_Death_Effect.Melee_Enemy_Death_Effect" (+ _returnvalue "0, 0,20.000000"))
  (Actor|DestroyActor)
  (bind _asghost_player (Utilities|Casting|CastToGhost_Player (Game|GetPlayerCharacter 0)))
  (Default|AddStreak _asghost_player)
  (Default|AddPoints _asghost_player (+ 9 (* (Math|Conversions|ToInteger(Boolean) (Variables|Default|GetElite)) 6)) true)
  (Variables|/Game/Blueprints/Ghost_Player.Ghost_Player_C|SetFleeting_Revolver_Live_Charge _asghost_player 1.0))

(event Custom|End_Hit
  ;[1 1 1] Hit
  (bind _asbase_enemy_controller (Utilities|Casting|CastToBase_Enemy_Controller (Pawn|GetController)))
  (Variables|/Game/Blueprints/AI_Enemies/Base_Enemy_Controller.Base_Enemy_Controller_C|SetState _asbase_enemy_controller "NewEnumerator0")
  (Default|UpdateState _asbase_enemy_controller))

(event EventBeginPlay
  ;[1 1 1] Hit
  (Variables|Default|SetGuard_Point (Transformation|GetWorldLocation (Variables|Character|GetMesh)))
  (Utilities|FlowControl|Delay 0.016 :!label _label)
  (Utilities|FlowControl|Sequence
    (:then_0
      (goto _label))
    (:then_1
      (Utilities|FlowControl|Gate true :!label _label_2
        (:Exit
          (for _array_element (Collision|GetOverlappingActors (Variables|Default|GetKilling_Capsule) "/Game/Blueprints/Ghost_Player.Ghost_Player_C" :!class /Script/Engine.PrimitiveComponent)
            (bind _asghost_player (Utilities|Casting|CastToGhost_Player _array_element))
            (if (Variables|/Game/Blueprints/Ghost_Player.Ghost_Player_C|GetShield_Active _asghost_player)
              (Default|AddPoints _asghost_player 14 true)
              (goto _label_2 Close)
              (else
                (Default|GetHit _asghost_player)
                (goto _label_2 Close)))))))))

(fn ConstructionScript
  (bind _mesh (Variables|Character|GetMesh))
  (bind _elite_marker (Variables|Default|GetElite_Marker))
  (bind _pointlight (Variables|Default|GetPointLight))
  (if (Variables|Default|GetElite)
    (Rendering|Material|SetMaterial _mesh 0 "/Game/Geometry/Mannequin/Character/Materials/M_Male_Body_Melee.M_Male_Body_Melee")
    (Rendering|SetVisibility _elite_marker true false)
    (Rendering|Components|Light|SetIntensity _pointlight 1.5e+04)
    (Class|PointLightComponent|SetSourceRadius _pointlight 0.0)
    (Class|PointLightComponent|SetSoftSourceRadius _pointlight 0.0)
    (else
      (Rendering|Material|SetMaterial _mesh 0 "/Game/Geometry/Mannequin/Character/Materials/M_Male_Body_Melee_Elite.M_Male_Body_Melee_Elite")
      (Rendering|SetVisibility _elite_marker false false)
      (Rendering|Components|Light|SetIntensity _pointlight 2.5e+03)
      (Class|PointLightComponent|SetSourceRadius _pointlight 1e+01)
      (Class|PointLightComponent|SetSoftSourceRadius _pointlight 1e+01))))