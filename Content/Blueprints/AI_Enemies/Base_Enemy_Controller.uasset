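; AI controller for enemies that runs Base_Enemy_BT and feeds its blackboard.
; BeginPlay sets a melee flag from the pawn class and writes State, which Update_State rewrites.
; Perception updates toggle Can_See_Player for Ghost_Player.
; Controller_Update_Gun aims the pawn's gun at the focused player's camera, with Elite enemies leading horizontal movement by a distance-scaled offset, and plays a one-time "Come On" sound.
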(event OnTargetPerceptionUpdated(AIPerception)
  (params (Actor :type Actor%20Object%20Reference) (Stimulus :type AI%20Stimulus%20Structure))
  (Utilities|Casting|CastToGhost_Player Actor)
  (AI|Components|Blackboard|SetValueasBool (AI|GetBlackboard 0) (Utilities|Name|MakeLiteralName "Can_See_Player") (.bSuccessfullySensed (Utilities|Struct|BreakAIStimulus Stimulus))))

(event Custom|Controller_Update_Gun
  (bind _self self)
  (Utilities|FlowControl|Sequence
    (:then_0
      (bind _asbase_enemy (Utilities|Casting|CastToBase_Enemy (Pawn|GetControlledPawn _self)))
      (bind _asghost_player (Utilities|Casting|CastToGhost_Player (Class|AIController|GetFocusActor _self)))
      (Default|UpdateGun _asbase_enemy (Math|Rotator|FindLookatRotation (Transformation|GetWorldLocation (Variables|/Game/Blueprints/AI_Enemies/Base_Enemy.Base_Enemy_C|GetGun_Rotation_Point _asbase_enemy)) (+ (Transformation|GetWorldLocation (Variables|/Game/Blueprints/Ghost_Player.Ghost_Player_C|GetFollowCamera _asghost_player)) (* (Math|Vector|Normalize (Math|Vector|MakeVector (.x (Transformation|GetVelocity _asghost_player)) (.y (Transformation|GetVelocity _asghost_player)) 0.0)) (select (Variables|/Game/Blueprints/AI_Enemies/Base_Enemy.Base_Enemy_C|GetElite _asbase_enemy) (/ (Transformation|GetDistanceTo _asghost_player _asbase_enemy) 6.0) 0.0))))))
    (:then_1
      ;[1 1 1] CAMOOON
      (Utilities|FlowControl|DoOnce false
        (:Completed
          (Audio|PlaySoundatLocation "/Game/Effects/Audio/Cue_Come_On.Cue_Come_On" (Transformation|GetActorLocation (Pawn|GetControlledPawn self)) "0, 0, 0" 1.0 1.0 0.0 0 0 0))))))

(event Custom|Update_State
  ;[1 1 1] Presettings
  (AI|Components|Blackboard|SetValueasEnum (AI|GetBlackboard 0) (Utilities|Name|MakeLiteralName "State") (Variables|Default|GetState)))

(event EventBeginPlay
  (bind _returnvalue (AI|GetBlackboard 0))
  (bind _returnvalue_2 (Pawn|GetControlledPawn))
  (bind _returnvalue_3 (Utilities|Name|MakeLiteralName "Is_Melee"))
  ;[1 1 1] Presettings
  (AI|RunBehaviorTree "/Game/Blueprints/AI_Enemies/Base_Enemy_BT.Base_Enemy_BT")
  (Utilities|FlowControl|Sequence
    (:then_0
      (Utilities|Casting|CastToBase_Enemy _returnvalue_2)
      (AI|Components|Blackboard|SetValueasBool _returnvalue _returnvalue_3 false))
    (:then_1
      (Utilities|Casting|CastToMelee_Enemy _returnvalue_2)
      (AI|Components|Blackboard|SetValueasBool _returnvalue _returnvalue_3 true))
    (:then_2
      (AI|Components|Blackboard|SetValueasEnum _returnvalue (Utilities|Name|MakeLiteralName "State") (Variables|Default|GetState)))))

(fn ConstructionScript)