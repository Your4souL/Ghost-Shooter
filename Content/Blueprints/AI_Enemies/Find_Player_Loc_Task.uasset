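; Behavior tree task that gives an enemy AI the Ghost_Player's location as its move target.
; If the player is falling, a downward visibility trace substitutes the ground point below for the actor location.
; It then sets a blackboard state enum by whether the player is within a fixed distance of the controlled pawn.
; The task fails when the player cast fails or the trace finds no hit.
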(event EventReceiveExecuteAI
  (params (OwnerController :type AI%20Controller%20Object%20Reference) (ControlledPawn :type Pawn%20Object%20Reference))
  (bind _asghost_player (Utilities|Casting|CastToGhost_Player (Game|GetPlayerCharacter 0))
    (:then
      (if (AI|Components|NavMovement|IsFalling (Variables|/Script/Engine.Character|GetCharacterMovement _asghost_player))
        (bind (_outhit _returnvalue) (Collision|LineTraceByChannel (Transformation|GetActorLocation _asghost_player) (+ (Transformation|GetActorLocation _asghost_player) (Math|Vector|MakeVector 0.0 0.0 -1e+04)) "TraceTypeQuery1" false (Utilities|Array|MakeArray _asghost_player) "None"))
        (if _returnvalue
          (AI|BehaviorTree|SetBlackboardValueasVector (Variables|Default|GetBB_Move_Target_Key) (.Location (Collision|BreakHitResult _outhit)))
          (Utilities|FlowControl|Sequence :!label _label
            (:then_0
              (Class|BTFunctionLibrary|SetBlackboardValueasEnum (Variables|Default|GetBB_State) (select (<= (Transformation|GetDistanceTo (Game|GetPlayerCharacter 0) ControlledPawn) 4.5e+02) "NewEnumerator1" "NewEnumerator0")))
            (:then_1
              (AI|BehaviorTree|FinishExecute true)))
          (else
            (AI|BehaviorTree|FinishExecute false)))
        (else
          (AI|BehaviorTree|SetBlackboardValueasVector (Variables|Default|GetBB_Move_Target_Key) (Transformation|GetActorLocation _asghost_player))
          (goto _label))))
    (:CastFailed
      (AI|BehaviorTree|FinishExecute false))))