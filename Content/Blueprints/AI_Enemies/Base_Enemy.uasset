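; Base enemy Blueprint for a gun-wielding foe with an optional Elite variant, set up in the construction script through materials, marker and light.
; It records its spawn location as a guard point and exposes events to rotate the gun and fire.
; Shooting is a delay-timed sequence of charge effects, sound and a pulsed revolver barrel.
; Self-destruct spawns death effects, then awards the player streak, Elite-weighted points and revolver charge.
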(event Custom|Shoot
  (bind _revolver_ebbarrel (Variables|Default|GetRevolver_EBBarrel))
  (bind _base_charge_system (Variables|Default|GetBase_Charge_System))
  (bind _shoot_system (Variables|Default|GetShoot_System))
  (Components|Activation|SetActive _base_charge_system true true)
  (Utilities|FlowControl|Delay 0.975)
  (Components|Activation|Activate _shoot_system false)
  (Utilities|FlowControl|Delay 0.025)
  (Class|EBBarrel|Shoot _revolver_ebbarrel true)
  (Audio|PlaySoundatLocation "/Game/Effects/Audio/Revolver/Cue_Revolver.Cue_Revolver" (Transformation|GetWorldLocation _revolver_ebbarrel) "0, 0, 0" 1.0 1.0 0.0 "/Game/Effects/Audio/Base_Dir_Attenuation.Base_Dir_Attenuation" 0 0)
  (Utilities|FlowControl|Delay 0.0)
  (Class|EBBarrel|Shoot _revolver_ebbarrel false)
  (Components|Activation|SetActive _base_charge_system false true)
  (Utilities|FlowControl|Delay 1.0)
  (Components|Activation|Deactivate _shoot_system))

(event Custom|Update_Gun
  (params (New_Rotation :type Rotator))
  (Transformation|SetWorldRotation (Variables|Default|GetGun_Rotation_Point) New_Rotation false false))

(event Custom|Self_Distruct
  (bind _mesh (Variables|Character|GetMesh))
  (bind _returnvalue (Transformation|GetWorldLocation _mesh))
  (Audio|PlaySoundatLocation "/Game/Effects/Audio/Soul_Pha_Cue.Soul_Pha_Cue" _returnvalue "0, 0, 0" 1.0 1.0 0.0 "/Game/Effects/Audio/Base_Dir_Attenuation.Base_Dir_Attenuation" 0 0)
  (Niagara|SpawnSystematLocation "/Game/Effects/Base_Enemy_Death_Effect.Base_Enemy_Death_Effect" (+ _returnvalue "0, 0,20.000000"))
  (Actor|DestroyActor)
  (bind _asghost_player (Utilities|Casting|CastToGhost_Player (Game|GetPlayerCharacter 0)))
  (Default|AddStreak _asghost_player)
  (Default|AddPoints _asghost_player (+ 7 (* (Math|Conversions|ToInteger(Boolean) (Variables|Default|GetElite)) 4)) true)
  (Variables|/Game/Blueprints/Ghost_Player.Ghost_Player_C|SetFleeting_Revolver_Live_Charge _asghost_player 1.0))

(event EventBeginPlay
  (Variables|Default|SetGuard_Point (Transformation|GetWorldLocation (Variables|Character|GetMesh))))

(fn ConstructionScript
  (bind _mesh (Variables|Character|GetMesh))
  (bind _elite_marker (Variables|Default|GetElite_Marker))
  (bind _pointlight (Variables|Default|GetPointLight))
  (if (Variables|Default|GetElite)
    (Rendering|Material|SetMaterial _mesh 0 "/Game/Geometry/Mannequin/Character/Materials/M_Male_Body_Alt.M_Male_Body_Alt")
    (Rendering|SetVisibility _elite_marker true false)
    (Rendering|Components|Light|SetIntensity _pointlight 1.5e+04)
    (Class|PointLightComponent|SetSourceRadius _pointlight 0.0)
    (Class|PointLightComponent|SetSoftSourceRadius _pointlight 0.0)
    (else
      (Rendering|Material|SetMaterial _mesh 0 "/Game/Geometry/Mannequin/Character/Materials/M_Male_Body_Easy.M_Male_Body_Easy")
      (Rendering|SetVisibility _elite_marker false false)
      (Rendering|Components|Light|SetIntensity _pointlight 2.5e+03)
      (Class|PointLightComponent|SetSourceRadius _pointlight 1e+01)
      (Class|PointLightComponent|SetSoftSourceRadius _pointlight 1e+01))))